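; Right-side counter collision Blueprint that displays dirty and washed plate text.
; Four custom events let external callers set the string and toggle the visibility of the DirtyPlatesText and WashedPlatesText components separately.
; Strings are converted to Text, and visibility changes do not propagate to child components.
; It holds no plate-counting or overlap logic; BeginOverlap, Tick and the construction script are empty.
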(event `SetDirtyPlatesText`
  (params (DirtyPlatesString :type String))
  (`TextRenderComponent.K2_SetText` (`self.DirtyPlatesText`) (`KismetTextLibrary.Conv_StringToText` DirtyPlatesString)))

(event `SetDirtyPlatesTextVisibility`
  (params (DirtyPlatesVisible :type Boolean))
  (`SceneComponent.SetVisibility` (`self.DirtyPlatesText`) DirtyPlatesVisible false))

(event `SetWashedPlatesText`
  (params (WashedPlatesString :type String))
  (`TextRenderComponent.K2_SetText` (`self.WashedPlatesText`) (`KismetTextLibrary.Conv_StringToText` WashedPlatesString)))

(event `SetWashedPlatesTextVisibility`
  (params (WashedPlatesVisible :type Boolean))
  (`SceneComponent.SetVisibility` (`self.WashedPlatesText`) WashedPlatesVisible false))

(fn `UserConstructionScript`)