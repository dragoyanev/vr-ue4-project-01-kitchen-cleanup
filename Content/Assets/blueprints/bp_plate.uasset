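; Plate actor that can be picked up, dropped and cleaned away by a restart button.
; On BeginPlay it finds the first Bp_buttonrestart and binds to its clean-plates event, which plays a clank sound at the mesh and destroys the plate.
; PickUp disables mesh physics and attaches the root to the given target; DropOff re-enables physics and detaches.
; HitSurface is an empty stub.
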(event `self.ReceiveBeginPlay`
  (bind _outactors (`GameplayStatics.GetAllActorsOfClass` "/Game/Assets/blueprints/bp_buttonrestart.bp_buttonrestart_C"))
  (bind _output_get (set `self.buttonRestart` (`KismetArrayLibrary.Array_Get` _outactors)))
  (add `/Game/Assets/blueprints/bp_buttonrestart.cleanPlates` _output_get (delegate `Cleaned`)))

(event `Cleaned`
  (`GameplayStatics.PlaySoundAtLocation` "/Game/Assets/audio/kitchen_plate_clank_Cue.kitchen_plate_clank_Cue" (`SceneComponent.K2_GetComponentLocation` (`self.plate_mesh`)))
  (`self.K2_DestroyActor`))

(event `/Game/Assets/blueprints/PickUpAbleInterface.pickUp`
  (params (ActorToAttachTo :type "SceneComponent Object Reference"))
  (`PrimitiveComponent.SetSimulatePhysics` (`self.plate_mesh`) false)
  (`SceneComponent.K2_AttachToComponent` (`self.K2_GetRootComponent`) ActorToAttachTo "None" "KeepWorld" "KeepWorld" "KeepWorld" true))

(event `HitSurface`)

(event `/Game/Assets/blueprints/PickUpAbleInterface.dropOff`
  (`PrimitiveComponent.SetSimulatePhysics` (`self.plate_mesh`) true)
  (`self.K2_DetachFromActor` "KeepWorld" "KeepWorld" "KeepWorld"))

(fn `UserConstructionScript`)